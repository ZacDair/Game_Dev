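; Basic AI enemy that spots players and fires shots.
; On perception updates, if the Blackboard has no valid Player, it stores the first sighted FirstPersonCharacter whose MyPlayerState Health is nonzero.
; Tick polls IsAttacking, spawns an actor from the eye viewpoint, plays a quiet fire sound and resets the flag, so each trigger yields one shot.
; Nothing here sets that flag or clears the target.
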(event OnPerceptionUpdated(AIPerception)
  (params (UpdatedActors :type Array%20of%20Actor%20Object%20References))
  (bind _returnvalue (Utilities|Name|MakeLiteralName "Player"))
  (bind _returnvalue_2 (AI|GetBlackboard 0))
  (Utilities|IsValid (AI|Components|Blackboard|GetValueasObject _returnvalue_2 _returnvalue)
    (:Is%20Not%20Valid
      (bind _array_element (Utilities|Array|ForEachLoopwithBreak (Class|AIPerceptionComponent|GetCurrentlyPerceivedActors (Variables|Default|GetAIPerception) "/Script/AIModule.AISense_Sight") :!label _label)
        (:LoopBody
          (bind _asfirst_person_character (Utilities|Casting|CastToFirstPersonCharacter _array_element))
          (bind _asmy_player_state (Utilities|Casting|CastToMyPlayerState (Variables|/Script/Engine.Pawn|GetPlayerState _asfirst_person_character)))
          (if (not (== (Variables|/Game/Blueprints/MyPlayerState.MyPlayerState_C|GetHealth _asmy_player_state) 0.0))
            (AI|Components|Blackboard|SetValueasObject _returnvalue_2 _returnvalue _asfirst_person_character)
            (goto _label Break)))))))

(event Custom|CustomEvent
  (params (DeltaSeconds :type Float%20%28single-precision%29)))

(event EventBeginPlay)

(event EventTick
  (params (DeltaSeconds :type Float%20%28single-precision%29))
  (bind (_outlocation _outrotation) (Actor|GetActorEyesViewPoint))
  (if (Variables|Default|GetisAttacking?)
    (Game|SpawnActorfromClass "/Game/FirstPersonBP/Blueprints/Projectiles/YellowProjectile.YellowProjectile_C" (Math|Transform|MakeTransform _outlocation _outrotation) "AdjustIfPossibleButDontSpawnIfColliding" 0 0)
    (Audio|PlaySoundatLocation "/Game/FirstPerson/Audio/FirstPersonTemplateWeaponFire02.FirstPersonTemplateWeaponFire02" (Transformation|GetActorLocation) "0, 0, 0" 0.01 1.0 0.0 0 0 0) ; Play firing sound
    (Variables|Default|SetisAttacking? false)))

(event Collision|EventActorBeginOverlap
  (params (OtherActor :type Actor%20Object%20Reference)))

(fn ConstructionScript
  (|CallParentFunction))