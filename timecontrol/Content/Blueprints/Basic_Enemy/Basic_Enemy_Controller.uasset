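; AI controller for the basic enemy that runs its behavior tree on BeginPlay and picks a player to target by sight.
; On perception updates, if the Blackboard's Player key has no valid object, it scans sight-perceived actors for a FirstPersonCharacter with non-zero Health in its MyPlayerState.
; The first match is written to the Player key, which this controller never clears.
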(event OnPerceptionUpdated(AIPerception)
  (params (UpdatedActors :type Array%20of%20Actor%20Object%20References))
  (bind _returnvalue (Utilities|Name|MakeLiteralName "Player"))
  (bind _returnvalue_2 (AI|GetBlackboard 0))
  ;[1 1 1] Detect a player using sight and expose the actor to the Blackboard
  (Utilities|IsValid (AI|Components|Blackboard|GetValueasObject _returnvalue_2 _returnvalue)
    (:Is%20Not%20Valid
      (bind _array_element (Utilities|Array|ForEachLoopwithBreak (Class|AIPerceptionComponent|GetCurrentlyPerceivedActors (Variables|Default|GetAIPerception) "/Script/AIModule.AISense_Sight") :!label _label)
        (:LoopBody
          (bind _asfirst_person_character (Utilities|Casting|CastToFirstPersonCharacter _array_element))
          (bind _asmy_player_state (Utilities|Casting|CastToMyPlayerState (Variables|/Script/Engine.Pawn|GetPlayerState _asfirst_person_character)))
          (if (not (== (Variables|/Game/Blueprints/MyPlayerState.MyPlayerState_C|GetHealth _asmy_player_state) 0.0))
            (AI|Components|Blackboard|SetValueasObject _returnvalue_2 _returnvalue _asfirst_person_character)
            (goto _label Break)))))))

(event EventBeginPlay
  (AI|RunBehaviorTree "/Game/Blueprints/Basic_Enemy/Basic_Enemy_BTree.Basic_Enemy_BTree"))

(fn ConstructionScript)