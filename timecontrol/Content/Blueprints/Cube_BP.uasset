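; Physics cube that can rewind its motion, switched by Rewind and Forward events.
; While playing forward, Tick records the mesh's world transform and its velocities, packing linear and angular velocity into a Transform's Location and Scale.
; While rewinding, it pops both uncapped histories frame by frame, restoring the transform and applying negated, halved velocities.
; At the oldest sample it holds that transform; the start location and rotation saved on BeginPlay go unused.
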(event EventBeginPlay
  (bind _mesh (Variables|Default|GetMesh))
  (Variables|Default|SetstartingLocation (Transformation|GetWorldLocation _mesh))
  (Variables|Default|SetstartingRotation (Transformation|GetWorldRotation _mesh)))

(event EventRewind
  (Variables|Default|SetRewinding true))

(event EventForward
  (Variables|Default|SetRewinding false))

(event EventTick
  (params (DeltaSeconds :type Float%20%28single-precision%29))
  (bind _mesh (Variables|Default|GetMesh))
  (bind _mesh_2 (Variables|Default|GetMesh))
  (bind _actorvelocities (Variables|Default|GetActorVelocities))
  (bind _actorvelocities_2 (Variables|Default|GetActorVelocities))
  (bind _actortransforms (Variables|Default|GetActorTransforms))
  (bind _actortransforms_2 (Variables|Default|GetActorTransforms))
  (bind _actortransforms_3 (Variables|Default|GetActorTransforms))
  (bind _returnvalue (Utilities|Array|LastIndex _actortransforms))
  (bind _returnvalue_2 (Utilities|Array|LastIndex _actortransforms_3))
  (bind _returnvalue_3 (Utilities|Array|LastIndex _actorvelocities))
  (bind _returnvalue_4 (Utilities|Array|LastIndex _actorvelocities_2))
  (bind _output (Utilities|Array|Get(acopy) _actorvelocities _returnvalue_3))
  (bind (_location _rotation _scale) (Math|Transform|BreakTransform _output))
  (Utilities|FlowControl|Sequence
    (:then_0
      (if (Variables|Default|GetRewinding)
        (if (> _returnvalue_2 0)
          (Transformation|SetWorldTransform (Variables|Default|GetMesh) (Utilities|Array|Get(acopy) _actortransforms_3 _returnvalue_2) false false)
          (if (> _returnvalue 0)
            (Utilities|Array|RemoveIndex _actortransforms _returnvalue))
          (else
            (Transformation|SetWorldTransform (Variables|Default|GetMesh) (Utilities|Array|Get(acopy) _actortransforms_2 (Utilities|Array|LastIndex _actortransforms_2)) false false)))
        (else
          (Utilities|Array|Add (Variables|Default|GetActorTransforms) (Transformation|GetWorldTransform (Variables|Default|GetMesh))))))
    (:then_1
      (if (Variables|Default|GetRewinding)
        (if (> (Utilities|Array|LastIndex (Variables|Default|GetActorVelocities)) 0)
          (Physics|SetPhysicsLinearVelocity _mesh_2 (/ (Math|Vector|NegateVector _location) 2) false "None")
          (Class|PrimitiveComponent|SetPhysicsAngularVelocityinDegrees _mesh_2 (/ (Math|Vector|NegateVector _scale) 2) false "None")
          (if (> _returnvalue_4 0)
            (Utilities|Array|RemoveIndex _actorvelocities_2 _returnvalue_4)))
        (else
          (bind _returnvalue_5 (Physics|GetPhysicsLinearVelocity _mesh "None"))
          (Utilities|Array|Add (Variables|Default|GetActorVelocities) (Math|Transform|MakeTransform _returnvalue_5 "0, 0, 0" (Physics|GetPhysicsAngularVelocityinDegrees _mesh "None"))))))))

(fn ConstructionScript)