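; An AI character that chases the player and can rewind its own movement through time.
; BeginPlay loops AI MoveTo toward player 0, retrying shortly after success or failure.
; Each Tick records the transform and physics velocities in uncapped arrays, or pops and applies the newest entries while the Rewind event's flag is set until Forward clears it.
; Velocities are packed into Transforms, linear in Location and angular in Scale.
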(event EventRewind
  ;[1 1 1] Set our rewinding val based on the event called
  (Variables|Default|SetRewinding true))

(event EventForward
  ;[1 1 1] Set our rewinding val based on the event called
  (Variables|Default|SetRewinding false))

(event EventTick
  (params (DeltaSeconds :type Float%20%28single-precision%29))
  (bind _actorvelocities (Variables|Default|GetActorVelocities))
  (bind _actorvelocities_2 (Variables|Default|GetActorVelocities))
  (bind _charactermovement (Variables|Character|GetCharacterMovement))
  (bind _actortransforms (Variables|Default|GetActorTransforms))
  (bind _actortransforms_2 (Variables|Default|GetActorTransforms))
  (bind _actortransforms_3 (Variables|Default|GetActorTransforms))
  (bind _charactermovement_2 (Variables|Character|GetCharacterMovement))
  (bind _returnvalue (Utilities|Array|LastIndex _actortransforms))
  (bind _returnvalue_2 (Utilities|Array|LastIndex _actortransforms_3))
  (bind _returnvalue_3 (Utilities|Array|LastIndex _actorvelocities))
  (bind _returnvalue_4 (Utilities|Array|LastIndex _actorvelocities_2))
  (bind _updatedprimitive (Variables|/Script/Engine.MovementComponent|GetUpdatedPrimitive _charactermovement))
  (bind _updatedprimitive_2 (Variables|/Script/Engine.MovementComponent|GetUpdatedPrimitive _charactermovement_2))
  (bind _output (Utilities|Array|Get(acopy) _actorvelocities _returnvalue_3))
  (bind (_location _rotation _scale) (Math|Transform|BreakTransform _output))
  (Utilities|FlowControl|Sequence
    (:then_0
      (if (Variables|Default|GetRewinding)
        (if (> _returnvalue_2 0)
          (Transformation|SetActorTransform (Utilities|Array|Get(acopy) _actortransforms_3 _returnvalue_2))
          (if (> _returnvalue 0)
            (Utilities|Array|RemoveIndex _actortransforms _returnvalue))
          (else
            (Transformation|SetActorTransform (Utilities|Array|Get(acopy) _actortransforms_2 (Utilities|Array|LastIndex _actortransforms_2)))))
        (else
          (Utilities|Array|Add (Variables|Default|GetActorTransforms) (Transformation|GetActorTransform self)))))
    (:then_1
      (if (Variables|Default|GetRewinding)
        (if (> (Utilities|Array|LastIndex (Variables|Default|GetActorVelocities)) 0)
          (Physics|SetPhysicsLinearVelocity _updatedprimitive_2 _location false "None")
          (Class|PrimitiveComponent|SetPhysicsAngularVelocityinDegrees _updatedprimitive_2 _scale false "None")
          (if (> _returnvalue_4 0)
            (Utilities|Array|RemoveIndex _actorvelocities_2 _returnvalue_4)))
        (else
          (bind _returnvalue_5 (Physics|GetPhysicsLinearVelocity _updatedprimitive "None"))
          (Utilities|Array|Add (Variables|Default|GetActorVelocities) (Math|Transform|MakeTransform _returnvalue_5 "0, 0, 0" (Physics|GetPhysicsAngularVelocityinDegrees _updatedprimitive "None"))))))))

(event EventBeginPlay
  ;[1 1 1] Move to player
  (AI|AIMoveTo self "0, 0, 0" (Game|GetPlayerCharacter 0) 5.0 false :!label _label
    (:OnSuccess
      _)
    (:OnFail
      _))
  (Utilities|FlowControl|Delay 0.2)
  (goto _label))

(fn ConstructionScript)